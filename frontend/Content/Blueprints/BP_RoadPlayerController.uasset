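; Player controller for a road editor that shows the editor UI and mouse cursor and links to BP_RoadEditorManager.
; Left click follows the build mode: Straight forwards the click to the manager, while Bezier Curve stores the cursor's hit location.
; Enter ends the current road segment through the manager and switches the UI panel.
; GetBezierPoint evaluates a cubic Bezier with nested lerps, but nothing here calls it.
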(event `Key|LeftMouseButton`
  (params (Key :type "Key Structure"))
  (:`Pressed`
    (switch `/Game/Blueprints/E_RoadBuildMode` (`self.CurrentBuildMode`)
      (:`NewEnumerator0`
        (`RoadEditorManager.HandleMouseClick` (`self.ManagerRef`)))
      (:`NewEnumerator1`
        (`KismetArrayLibrary.Array_Add` (`self.BeizerClickPoints`) (`.Location` (`GameplayStatics.BreakHitResult` (`self.GetHitResultUnderCursorByChannel` "TraceTypeQuery1"))))))))

(event `Key|Enter`
  (params (Key :type "Key Structure"))
  (:`Pressed`
    (`RoadEditorManager.EndCurrentRoadSegment` (`self.ManagerRef`))
    (`WidgetSwitcher.SetActiveWidgetIndex` (`/Game/Blueprints/WBP_RoadEditorUI.PanelSwitcher` (`self.UIRef`)) 1)))

(event `self.ReceiveBeginPlay`
  (bind _returnvalue (`|CreateWidget` "/Game/Blueprints/WBP_RoadEditorUI.WBP_RoadEditorUI_C" (`GameplayStatics.GetPlayerController` 0)))
  (set `self.UIRef` _returnvalue)
  (`UserWidget.AddToViewport` _returnvalue 0)
  (set `self.bShowMouseCursor` true)
  (bind _returnvalue_2 (`GameplayStatics.GetActorOfClass` "/Game/Blueprints/BP_RoadEditorManager.BP_RoadEditorManager_C"))
  (set `self.ManagerRef` _returnvalue_2))

(fn `GetBezierPoint`
  (params (P0 :type "Vector Structure") (P1 :type "Vector Structure") (P2 :type "Vector Structure") (P3 :type "Vector Structure") (T :type "Float (double-precision)"))
  (returns (CalculatedPoint :type "Vector Structure"))
  (bind _returnvalue (`KismetMathLibrary.VLerp` P1 P2 T))
  (return (`KismetMathLibrary.VLerp` (`KismetMathLibrary.VLerp` (`KismetMathLibrary.VLerp` P0 P1 T) _returnvalue T) (`KismetMathLibrary.VLerp` _returnvalue (`KismetMathLibrary.VLerp` P2 P3 T) T) T)))

(fn `UserConstructionScript`)