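; BP_SimCameraPawn is a camera pawn that follows one selected instance of an instanced static mesh.
; Each Tick, when TargetIndex is non-negative and TargetISM is valid, it reads that instance's world-space transform.
; It eases its own location and rotation toward that transform with VInterpTo and RInterpTo, both driven by CameraPanSpeed.
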(event `self.ReceiveTick`
  (params (DeltaSeconds :type "Float (single-precision)"))
  (bind _returnvalue (`GameplayStatics.GetWorldDeltaSeconds`))
  (bind _camerapanspeed (`self.CameraPanSpeed`))
  (if (>= (`self.TargetIndex`) 0)
    (bind _targetism (`self.TargetISM`)
      (:`then`
        (bind _outinstancetransform (`InstancedStaticMeshComponent.GetInstanceTransform` _targetism (`self.TargetIndex`) true))
        (`self.K2_SetActorLocationAndRotation` (`KismetMathLibrary.VInterpTo` (`self.K2_GetActorLocation`) (.location _outinstancetransform) _returnvalue _camerapanspeed) (`KismetMathLibrary.RInterpTo` (`self.K2_GetActorRotation`) (.rotation _outinstancetransform) _returnvalue _camerapanspeed)))
      (:`else`))))

(fn `UserConstructionScript`)