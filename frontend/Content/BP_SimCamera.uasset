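; Player-controlled camera pawn for viewing a vehicle simulation, with move, drag-pan, rotate and zoom through Enhanced Input.
; Tick eases spring arm length and yaw toward input-set targets; TargetPitch is computed but never applied.
; Clicking a SimulationManager mesh instance opens a stats widget and locks the camera to that vehicle.
; Tick re-resolves the vehicle ID to its instance index to follow it, until Space or its disappearance releases it.
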(event `self.ReceiveTick`
  (params (DeltaSeconds :type "Float (single-precision)"))
  (bind _springarm (`self.SpringArm`))
  (bind _simmanagerref (`self.SimManagerRef`))
  (bind (_returnvalue_roll _returnvalue_pitch) (`KismetMathLibrary.BreakRotator` (`SceneComponent.K2_GetComponentRotation` _springarm)))
  (set `SpringArmComponent.TargetArmLength` (`KismetMathLibrary.FInterpTo` (`SpringArmComponent.TargetArmLength` _springarm) (`self.TargetArmLength`) DeltaSeconds 4.5) _springarm)
  (`SceneComponent.K2_SetWorldRotation` _springarm (`KismetMathLibrary.RInterpTo` (`SpringArmComponent.GetTargetRotation` _springarm) (`KismetMathLibrary.MakeRotator` 0.0 _returnvalue_pitch (`self.TargetYaw`)) DeltaSeconds 4.5) false false)
  (`/Engine/EditorBlueprintResources/StandardMacros.IsValid` (`self.ActiveVehicleWidget`)
    (:`Is Valid`
      (`/Engine/EditorBlueprintResources/StandardMacros.IsValid` _simmanagerref
        (:`Is Valid`
          (bind _returnvalue (`SimulationManager.GetInstanceIndexFromVehicleID` _simmanagerref (`self.TargetVehicleID`)))
          (if (>= _returnvalue 0)
            (bind (_outstats _returnvalue_2) (`SimulationManager.GetVehicleStatsFromInstance` _simmanagerref _returnvalue))
            (if _returnvalue_2
              (`/Game/WBP_VehicleStats.UpdateStatsUI` (`self.ActiveVehicleWidget`) _outstats)
              (if (`self.bsIsCameraLocked`)
                (bind _returnvalue_3 (`SimulationManager.GetInstanceIndexFromVehicleID` _simmanagerref (`self.TargetVehicleID`)))
                (`self.K2_SetActorLocation` (.location (`InstancedStaticMeshComponent.GetInstanceTransform` (`self.GetComponentByClass` _simmanagerref "/Script/Engine.InstancedStaticMeshComponent") _returnvalue_3 true)))))
            (else
              (`Widget.RemoveFromParent` (`self.ActiveVehicleWidget`))
              (set `self.bsIsCameraLocked` false))))))))

(event `EnhancedInput|/Game/IA_Move`
  (params (ActionValue :type "Vector2D Structure") (ElapsedSeconds :type "Float (double-precision)") (TriggeredSeconds :type "Float (double-precision)") (InputAction :type "InputAction Object Reference" :default "/Game/IA_Move.IA_Move"))
  (bind (_returnvalue_roll _returnvalue_pitch _returnvalue_yaw) (`KismetMathLibrary.BreakRotator` (`SceneComponent.K2_GetComponentRotation` (`self.SpringArm`))))
  (bind _returnvalue (`KismetMathLibrary.MakeRotator` 0.0 0.0 _returnvalue_yaw))
  (:`Triggered`
    (`self.AddMovementInput` (`KismetMathLibrary.GetForwardVector` _returnvalue) ActionValue_X)
    (`self.AddMovementInput` (`KismetMathLibrary.GetRightVector` _returnvalue) ActionValue_Y)))

(event `EnhancedInput|/Game/IA_ActivateRotate`
  (params (ActionValue :type Boolean) (ElapsedSeconds :type "Float (double-precision)") (TriggeredSeconds :type "Float (double-precision)") (InputAction :type "InputAction Object Reference" :default "/Game/IA_ActivateRotate.IA_ActivateRotate"))
  (:`Started`
    (set `self.IsRotating` true))
  (:`Completed`
    (set `self.IsRotating` false)))

(event `self.ReceivePossessed`
  (params (NewController :type "Controller Object Reference"))
  (bind (_returnvalue_roll _returnvalue_pitch _returnvalue_yaw) (`KismetMathLibrary.BreakRotator` (`SceneComponent.K2_GetComponentRotation` (`self.SpringArm`))))
  (bind _asplayer_controller (cast `PlayerController` NewController))
  (`EnhancedInputSubsystemInterface.AddMappingContext` (pcsubsystem `EnhancedInputLocalPlayerSubsystem` _asplayer_controller) "/Game/IMC_SimControls.IMC_SimControls" 0 (struct))
  (set `self.TargetPitch` _returnvalue_pitch)
  (set `self.TargetYaw` _returnvalue_yaw))

(event `EnhancedInput|/Game/IA_CameraLook`
  (params (ActionValue :type "Vector2D Structure") (ElapsedSeconds :type "Float (double-precision)") (TriggeredSeconds :type "Float (double-precision)") (InputAction :type "InputAction Object Reference" :default "/Game/IA_CameraLook.IA_CameraLook"))
  (:`Triggered`
    (if (`self.IsRotating`)
      (set `self.TargetYaw` (+ (`self.TargetYaw`) (* ActionValue_X 1.5)))
      (set `self.TargetPitch` (`KismetMathLibrary.FClamp` (+ ActionValue_Y (`self.TargetPitch`)) -35.0 -85.0)))))

(event `EnhancedInput|/Game/IA_Zoom`
  (params (ActionValue :type "Float (double-precision)") (ElapsedSeconds :type "Float (double-precision)") (TriggeredSeconds :type "Float (double-precision)") (InputAction :type "InputAction Object Reference" :default "/Game/IA_Zoom.IA_Zoom"))
  (:`Triggered`
    (bind _output_get (set `self.TargetArmLength` (`KismetMathLibrary.FClamp` (- (`self.TargetArmLength`) (* ActionValue 1500.0)) 5000.0 100000.0)))
    (set `self.TargetPitch` (`KismetMathLibrary.MapRangeClamped` _output_get 5000.0 100000.0 -35.0 -85.0))))

(event `EnhancedInput|/Game/IA_ActivateDrag`
  (params (ActionValue :type Boolean) (ElapsedSeconds :type "Float (double-precision)") (TriggeredSeconds :type "Float (double-precision)") (InputAction :type "InputAction Object Reference" :default "/Game/IA_ActivateDrag.IA_ActivateDrag"))
  (:`Started`
    (set `self.IsDragging` true))
  (:`Completed`
    (set `self.IsDragging` false)))

(event `EnhancedInput|/Game/IA_DragPan`
  (params (ActionValue :type "Vector2D Structure") (ElapsedSeconds :type "Float (double-precision)") (TriggeredSeconds :type "Float (double-precision)") (InputAction :type "InputAction Object Reference" :default "/Game/IA_DragPan.IA_DragPan"))
  (bind (_returnvalue_roll _returnvalue_pitch _returnvalue_yaw) (`KismetMathLibrary.BreakRotator` (`SceneComponent.K2_GetComponentRotation` (`self.SpringArm`))))
  (bind _returnvalue (* (`self.TargetArmLength`) 0.01))
  (bind _returnvalue_2 (`KismetMathLibrary.MakeRotator` 0.0 0.0 _returnvalue_yaw))
  (:`Triggered`
    (if (`self.IsDragging`)
      (`self.K2_AddActorWorldOffset` (+ (* (`KismetMathLibrary.GetForwardVector` _returnvalue_2) (* ActionValue_Y _returnvalue)) (* (`KismetMathLibrary.GetRightVector` _returnvalue_2) (* ActionValue_X _returnvalue)))))))

(event `EnhancedInput|/Game/IA_Click`
  (params (ActionValue :type Boolean) (ElapsedSeconds :type "Float (double-precision)") (TriggeredSeconds :type "Float (double-precision)") (InputAction :type "InputAction Object Reference" :default "/Game/IA_Click.IA_Click"))
  (bind _activevehiclewidget (`self.ActiveVehicleWidget`))
  (bind (_bblockinghit _binitialoverlap _time _distance _location _impactpoint _normal _impactnormal _physmat _hitactor _hitcomponent _hitbonename _bonename _hititem) (`GameplayStatics.BreakHitResult` (`PlayerController.GetHitResultUnderCursorByChannel` (`GameplayStatics.GetPlayerController` 0) "TraceTypeQuery1" true)))
  (:`Triggered`
    (bind _assimulation_manager (cast `SimulationManager` _hitactor))
    (bind _output_get (set `self.SimManagerRef` _assimulation_manager))
    (bind (_outstats _returnvalue) (`SimulationManager.GetVehicleStatsFromInstance` _output_get _hititem))
    (if _returnvalue
      (set `self.TargetVehicleID` (`.VehicleID` (break `VehicleIDMStats` _outstats)))
      (`/Engine/EditorBlueprintResources/StandardMacros.IsValid` _activevehiclewidget
        (:`Is Valid`
          (`Widget.RemoveFromParent` _activevehiclewidget))
        (:`Is Not Valid`
          _))
      (bind _returnvalue_2 (`|CreateWidget` "/Game/WBP_VehicleStats.WBP_VehicleStats_C" null _outstats))
      (set `self.bsIsCameraLocked` true)
      (bind _output_get_2 (set `self.ActiveVehicleWidget` _returnvalue_2))
      (`UserWidget.AddToViewport` _output_get_2 0))))

(event `Key|SpaceBar`
  (params (Key :type "Key Structure"))
  (bind _activevehiclewidget (`self.ActiveVehicleWidget`))
  (:`Pressed`
    (set `self.bsIsCameraLocked` false)
    (`/Engine/EditorBlueprintResources/StandardMacros.IsValid` _activevehiclewidget
      (:`Is Valid`
        (`Widget.RemoveFromParent` _activevehiclewidget)))))

(fn `UserConstructionScript`)